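; BP_DragonEgg is an interactable dragon egg that lets the player pick an element before it hatches.
; Interact pauses the game and opens the WBP_DragonElement widget with a reference to the egg and mouse input enabled.
; PlayHatch restores gameplay input, plays the egg animation and makes it ignore pawn collision.
; It then passes the selected element to FinishHatching and destroys the egg after a short delay.
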(event Custom|PlayHatch
  (params (SelectedElement :type EDragonElement%20Enum :default "None"))
  (bind _returnvalue (Game|GetPlayerController 0))
  (Game|SetGamePaused false)
  (Variables|/Script/Engine.PlayerController|SetbShowMouseCursor _returnvalue false)
  (Input|SetInputModeGameOnly _returnvalue false)
  (Audio|Components|Audio|Play (Variables|Default|GetEggMeshComponent) false)
  (Utilities|FlowControl|Delay 0.1)
  (Collision|SetCollisionProfileName (Variables|Default|GetEggMeshComponent) "IgnoreOnlyPawn" true :!class /Script/Engine.PrimitiveComponent)
  (Class|DragonEgg|FinishHatching SelectedElement)
  (Utilities|FlowControl|Delay 1.0)
  (Actor|DestroyActor))

(event EventInteract
  (params (Interactor :type Actor%20Object%20Reference))
  (bind _returnvalue (Game|GetPlayerController 0))
  (Game|SetGamePaused true)
  (bind _returnvalue_2 (UserInterface|CreateWidget "/Game/Blueprints/Widgets/WBP_DragonElement.WBP_DragonElement_C" _returnvalue self))
  (UserInterface|Viewport|AddtoViewport _returnvalue_2 0)
  (Variables|/Script/Engine.PlayerController|SetbShowMouseCursor _returnvalue true)
  (Input|SetInputModeGameandUI _returnvalue _returnvalue_2 "DoNotLock" true true))

(fn ConstructionScript)