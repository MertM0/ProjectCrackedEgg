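; Knight player character Blueprint that handles UI and attack animation playback.
; BeginPlay creates the HUD, which also displays interaction warnings through an event.
; The U key flip-flops the stat upgrade widget, clearing the level-up text on open and switching pause, cursor and input mode.
; Montage events play a four-step light combo, selected by step index, or a heavy attack; combo logic itself lives outside this graph.
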(event EventPlayHeavyAttackMontage
  ;[0.15 0.15 0.15 0.5] Heavy Attack Anim Montage
  (Animation|PlayAnimMontage "/Game/Animations/Knight/Montages/AM_HeavyAttack.AM_HeavyAttack" 1.0 "None"))

(event EventBeginPlay
  (bind _returnvalue (UserInterface|CreateWidget "/Game/Blueprints/Widgets/WBP_HUD.WBP_HUD_C" (Game|GetPlayerController 0)))
  (bind _output_get (Variables|Default|SetHUD _returnvalue))
  (UserInterface|Viewport|AddtoViewport _returnvalue 0))

(event EventShowInteractionWarning
  (params (WarningMessage :type String))
  (Default|ShowWarningText (Variables|Default|GetHUD) (Utilities|Text|ToText(String) WarningMessage)))

(event EventPlayLightAttackMontage
  (params (ComboStep :type Integer))
  ;[0.15 0.15 0.15 0.5] Light Attack Anim Montages
  (switch int ComboStep
    (:1
      (Animation|PlayAnimMontage "/Game/Animations/Knight/Montages/AM_LightAttack_1.AM_LightAttack_1" 1.0 "None"))
    (:2
      (Animation|PlayAnimMontage "/Game/Animations/Knight/Montages/AM_LightAttack_2.AM_LightAttack_2" 1.0 "None"))
    (:3
      (Animation|PlayAnimMontage "/Game/Animations/Knight/Montages/AM_LightAttack_3.AM_LightAttack_3" 1.0 "None"))
    (:4
      (Animation|PlayAnimMontage "/Game/Animations/Knight/Montages/AM_LightAttack_4.AM_LightAttack_4" 1.0 "None"))))

(event Input|KeyboardEvents|U
  (params (Key :type Key%20Structure :default "None"))
  (bind _returnvalue (Game|GetPlayerController 0))
  ;[0.15 0.15 0.15 0.5] Stat Upgrade Widget
  (:Pressed
    (Utilities|FlowControl|FlipFlop
      (:A
        (bind _returnvalue_2 (UserInterface|CreateWidget "/Game/Blueprints/Widgets/WBP_StatUpgrade.WBP_StatUpgrade_C" _returnvalue))
        (UserInterface|Viewport|AddtoViewport _returnvalue_2 0)
        (Default|HideLevelUpText (Variables|Default|GetHUD))
        (Input|SetInputModeGameandUI _returnvalue _returnvalue_2 "DoNotLock" true true)
        (Variables|/Script/Engine.PlayerController|SetbShowMouseCursor _returnvalue true)
        (Game|SetGamePaused true))
      (:B
        (Widget|RemovefromParent _returnvalue_2)
        (Input|SetInputModeGameOnly _returnvalue true)
        (Variables|/Script/Engine.PlayerController|SetbShowMouseCursor _returnvalue false)
        (Game|SetGamePaused false)))))

(fn ConstructionScript)