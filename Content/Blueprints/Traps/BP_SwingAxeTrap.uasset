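; BP_SwingAxeTrap is a trap whose axe swings through an arc and hurts the knight.
; On BeginPlay the TM_Axe timeline drives the axe's relative rotation between two opposite angles, with an event track playing the swing sound.
; When a BP_Knight overlaps DamageBox, the trap calls DealDamage on it and plays a hit sound at the trap's location.
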(event OnComponentBeginOverlap(DamageBox)
  (params (OverlappedComponent :type Primitive%20Component%20Object%20Reference) (OtherActor :type Actor%20Object%20Reference) (OtherComp :type Primitive%20Component%20Object%20Reference) (OtherBodyIndex :type Integer) (bFromSweep :type Boolean) (SweepResult :type Hit%20Result%20Structure%20%28by%20ref%29))
  (bind _asbp_knight (Utilities|Casting|CastToBP_Knight OtherActor))
  (Class|BaseTrap|DealDamage _asbp_knight)
  (Audio|PlaySoundatLocation "/Game/Sounds/Traps/axe-hit.axe-hit" (Transformation|GetActorLocation) "0, 0, 0" 1.0 1.0 0.0 "/Game/Sounds/Attenuations/Default.Default" 0 0 0))

(event EventBeginPlay
  (bind _value (Timeline|TM_Axe Play)
    (:Update
      (Transformation|SetRelativeRotation (Variables|Default|GetAxe) (Math|Rotator|Lerp(Rotator) "-45.000000,0.000000,0.000000" "45.000000,0.000000,0.000000" _value) false false))
    (:Event
      (Audio|PlaySoundatLocation "/Game/Sounds/Traps/axe-swing.axe-swing" (Transformation|GetActorLocation) "0, 0, 0" 1.0 1.0 0.0 "/Game/Sounds/Attenuations/Default.Default" 0 0 0))))

(fn ConstructionScript)