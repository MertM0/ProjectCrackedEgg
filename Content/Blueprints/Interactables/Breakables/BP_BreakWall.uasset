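; BP_BreakWall is a breakable wall interactable that sets off fire particle effects when it starts to break.
; BeginPlay gathers six Fire components into a Particles array, and the OnBreakStarted event loops over that array to activate each one without a reset.
; The file holds only this effect hookup, with no break logic of its own and an empty construction script.
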(event EventOnBreakStarted
  (for _array_element (Variables|Default|GetParticles)
    (Components|Activation|Activate _array_element false)))

(event EventBeginPlay
  (Utilities|Array|Add (Variables|Default|GetParticles) (Variables|Default|Getfire1))
  (Utilities|Array|Add (Variables|Default|GetParticles) (Variables|Default|Getfire2))
  (Utilities|Array|Add (Variables|Default|GetParticles) (Variables|Default|Getfire3))
  (Utilities|Array|Add (Variables|Default|GetParticles) (Variables|Default|Getfire4))
  (Utilities|Array|Add (Variables|Default|GetParticles) (Variables|Default|Getfire5))
  (Utilities|Array|Add (Variables|Default|GetParticles) (Variables|Default|Getfire6)))

(fn ConstructionScript)