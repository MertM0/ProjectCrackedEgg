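; BP_BreakWall_Dragon is a breakable wall interactable that the player's dragon companion is sent to break.
; On interaction it finds the DragonCompanion actor and sets itself as that companion's priority target.
; BeginPlay gathers six fire particle components into an array.
; When breaking starts, it activates all of them, then plays the wall break sound at its location after a short delay.
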(event EventOnBreakStarted
  (for _array_element (Variables|Default|GetParticles)
    (Components|Activation|Activate _array_element false))
  (Utilities|FlowControl|Delay 0.5)
  (Audio|PlaySoundatLocation "/Game/Sounds/break-wall.break-wall" (Transformation|GetActorLocation) "0, 0, 0" 1.0 1.0 0.0 "/Game/Sounds/Attenuations/Default.Default" 0 0 0))

(event EventBeginPlay
  (Utilities|Array|Add (Variables|Default|GetParticles) (Variables|Default|Getfire1))
  (Utilities|Array|Add (Variables|Default|GetParticles) (Variables|Default|Getfire2))
  (Utilities|Array|Add (Variables|Default|GetParticles) (Variables|Default|Getfire3))
  (Utilities|Array|Add (Variables|Default|GetParticles) (Variables|Default|Getfire4))
  (Utilities|Array|Add (Variables|Default|GetParticles) (Variables|Default|Getfire5))
  (Utilities|Array|Add (Variables|Default|GetParticles) (Variables|Default|Getfire6)))

(event EventOnInteract
  (params (Interactor :type Actor%20Object%20Reference))
  (bind _returnvalue (Actor|GetActorOfClass "/Script/ProjectCrackedEgg.DragonCompanion"))
  (Class|DragonCompanion|SetPriorityTarget _returnvalue self))

(fn ConstructionScript)